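; Game mode that tracks coins and score, starts background music, and spawns a floating island at a random height on BeginPlay.
; Coins load from a CoinSave_BP save slot at start and are written back on EndPlay.
; When all enemies are defeated, Main_Map advances to Level_2_Map, while other levels show the supplied end-game widget with mouse input.
; A CameraShake event plays world camera shakes of a given type.
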(event `self.ReceiveBeginPlay`
  (`self.LoadCoins`)
  (`AudioComponent.Play` (`self.BGM`) 0.0)
  (`self.SpawnIsland`))

(event `self.ReceiveEndPlay`
  (params (EndPlayReason :type "EEndPlayReason Enum" :default "Destroyed"))
  (`self.SaveCoins`))

(event `CameraShake`
  (params (`Shake Type` :type "/Game/Blueprint/Camera_Shake_BP Class Reference"))
  (`GameplayStatics.PlayWorldCameraShake` `Shake Type` (0.0 0.0 0.0) -1.0 500.0))

(event `AllEnemiesDefeated`
  (params (`Widget to Show` :type "UserWidget Class Reference"))
  (bind _returnvalue (`GameplayStatics.GetCurrentLevelName` true))
  (if (`KismetStringLibrary.NotEqual_StrStr` _returnvalue "Main_Map")
    (bind _returnvalue_2 (`|CreateWidget` `Widget to Show`))
    (bind _output_get (set `self.Game Over Menu Reference` _returnvalue_2))
    (`UserWidget.AddToViewport` _output_get 0)
    (set `PlayerController.bShowMouseCursor` true (`GameplayStatics.GetPlayerController` 0))
    (set `PlayerController.bEnableMouseOverEvents` true (`GameplayStatics.GetPlayerController` 0))
    (`WidgetBlueprintLibrary.SetInputMode_GameAndUIEx` (`GameplayStatics.GetPlayerController` 0) null "DoNotLock" false)
    (else
      (`GameplayStatics.OpenLevel` "Level_2_Map"))))

(fn `Add Coin`
  (bind _output_get (set `self.coins` (+ (`self.coins`) 1)))
  (`KismetSystemLibrary.PrintString` (`KismetStringLibrary.BuildString_Int` "Coins:" " " _output_get)))

(fn `AddScore`
  (params (DeltaScore :type Integer))
  (set `self.score` (+ DeltaScore (`self.score`))))

(fn `LoadCoins`
  (bind _returnvalue (`GameplayStatics.DoesSaveGameExist` (`self.Coins Save Slot Name`)))
  (if _returnvalue
    (bind _returnvalue_2 (`GameplayStatics.LoadGameFromSlot` (`self.Coins Save Slot Name`)))
    (bind _output_get (set `self.Save Sub` _returnvalue_2))
    (bind _ascoin_save_bp (cast `/Game/Blueprint/CoinSave_BP` _output_get))
    (set `self.coins` (`/Game/Blueprint/CoinSave_BP.CoinCount` _ascoin_save_bp))
    (`GameplayStatics.SaveGameToSlot` (`self.Save Sub`) (`self.Coins Save Slot Name`))
    (else
      (`self.SaveCoins`))))

(fn `SaveCoins`
  (bind _returnvalue (`GameplayStatics.CreateSaveGameObject` "/Game/Blueprint/CoinSave_BP.CoinSave_BP_C"))
  (bind _output_get (set `self.Save Sub` _returnvalue))
  (bind _ascoin_save_bp (cast `/Game/Blueprint/CoinSave_BP` _output_get))
  (set `/Game/Blueprint/CoinSave_BP.CoinCount` (`self.coins`) _ascoin_save_bp)
  (`GameplayStatics.SaveGameToSlot` (`self.Save Sub`) (`self.Coins Save Slot Name`)))

(fn `SpawnIsland`
  (`|SpawnActorFromClass` "/Game/Blueprint/FloatingIsland_BP.FloatingIsland_BP_C" (`KismetMathLibrary.MakeTransform` (`KismetMathLibrary.MakeVector` 21000.0 35000.0 (`KismetMathLibrary.RandomFloatInRange` -2500.0 2500.0))) "Undefined" "OverrideRootScale" null null))

(fn `UserConstructionScript`)