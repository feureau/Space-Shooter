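; Base pickup Blueprint that drifts along the Y axis and homes in on the player pawn once it comes within range.
; A box collision overlap acts as the homing trigger, caching the first PlayerPawn_BP as the target.
; Each Tick blends ProjectileMovement velocity toward that pawn at an increased speed with a fixed lerp alpha, or keeps the default Y velocity without a valid target.
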(event `self.ReceiveTick`
  (params (DeltaSeconds :type "Float (single-precision)"))
  ;[1 1 1] Movement Control
  (`/Engine/EditorBlueprintResources/StandardMacros.IsValid` (`self.Player_Pawn_BP`)
    (:`Is Valid`
      (set `MovementComponent.Velocity` (`KismetMathLibrary.VLerp` (`MovementComponent.Velocity` (`self.ProjectileMovement`)) (* (`KismetMathLibrary.Normal` (- (`self.K2_GetActorLocation` (`self.Player_Pawn_BP`)) (`self.K2_GetActorLocation`))) (`self.Increased Speed`)) 0.1) (`self.ProjectileMovement`)))
    (:`Is Not Valid`
      (set `MovementComponent.Velocity` (`KismetMathLibrary.MakeVector` 0.0 (`self.Default Velocity`)) (`self.ProjectileMovement`)))))

(event `self.Box Collision.OnComponentBeginOverlap`
  (params (OverlappedComponent :type "PrimitiveComponent Object Reference") (OtherActor :type "Actor Object Reference") (OtherComp :type "PrimitiveComponent Object Reference") (OtherBodyIndex :type Integer) (bFromSweep :type Boolean) (SweepResult :type "HitResult Structure (by ref)"))
  ;[1 1 1] Homing radius control
  (bind _asplayer_pawn_bp (cast `/Game/Blueprint/Player_BP/PlayerPawn_BP` OtherActor))
  (`/Engine/EditorBlueprintResources/StandardMacros.IsValid` (`self.Player_Pawn_BP`)
    (:`Is Not Valid`
      (set `self.Player_Pawn_BP` _asplayer_pawn_bp))))

(fn `UserConstructionScript`)