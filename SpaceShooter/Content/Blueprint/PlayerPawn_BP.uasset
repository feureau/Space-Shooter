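; Player ship pawn for a shooter that moves in the Y-Z plane, with a timeline-driven fly-in on spawn.
; Tick applies interpolated input as swept movement and rolls the actor with vertical motion.
; Gates and countdown timers rate-limit held fire, choosing between a height-jittered primary shot and a multi-shot power-up.
; Both shots currently spawn PlayerPawn_BP itself, and rocket fire is an empty stub.
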(event `self.ReceiveBeginPlay`
  (bind _spawn_location (`self.spawn location`))
  (set `self.health` (`self.max health`))
  (set `self.pitch` (.pitch (`SceneComponent.RelativeRotation` (`self.Player Mesh`))))
  (set `self.spawn location` (`self.K2_GetActorLocation`))
  ;[1 1 1] Spawn Animation
  (bind (_direction _spawn) (`Timeline|Spawn Animation`)
    (:`Update`
      (`self.K2_SetActorLocation` (`KismetMathLibrary.VLerp` _spawn_location (+ _spawn_location (0.0 1000.0 0.0)) _spawn))
      (`SceneComponent.K2_SetRelativeRotation` (`self.Player Mesh`) (`KismetMathLibrary.RLerp` (struct) (`KismetMathLibrary.MakeRotator` 0.0 (+ (`self.Animation pitch`) (`self.pitch`))) _spawn) false false))))

(event `self.ReceiveTick`
  (params (DeltaSeconds :type "Float (single-precision)"))
  (set `self.delta seconds` DeltaSeconds)
  (if (`self.movement enabled`)
    (`self.Fire Rate Control`)
    (`|ExecutionSequence`
      (:`then_0`
        (bind _return_direction (`self.Get Direction` (`self.vertical speed`) (`self.GetInputAxisValue`)))
        (set `self.vertical speed` _return_direction))
      (:`then_1`
        (bind _return_direction_2 (`self.Get Direction` (`self.horizontal speed`) (`self.GetInputAxisValue`)))
        (set `self.horizontal speed` _return_direction_2))
      (:`then_2`
        (`self.K2_SetActorLocation` (+ (`self.K2_GetActorLocation`) (`KismetMathLibrary.MakeVector` 0.0 0.0 (`self.vertical speed`))) true)
        (`self.K2_SetActorLocation` (+ (`self.K2_GetActorLocation`) (`KismetMathLibrary.MakeVector` 0.0 (`self.horizontal speed`))) true)
        (set `self.vertical speed` (`self.GetInputAxisValue`))
        (set `self.horizontal speed` (`self.GetInputAxisValue`))
        (`self.K2_SetActorRotation` (`KismetMathLibrary.RInterpTo` (`self.K2_GetActorRotation`) (`KismetMathLibrary.MakeRotator` (* (`self.vertical speed`) -45.0) 0.0 90.0) (`self.delta seconds`) 5.0))))))

(event `InputAction|Primary Fire`
  (params (Key :type "Key Structure"))
  ;[1 1 1] Projectile Control
  (:`Pressed`
    (goto _label :!via `Open`))
  (:`Released`
    (goto _label :!via `Close`)))

(event `Fire Rate Control`
  ;[1 1 1] Projectile Control
  (`|ExecutionSequence`
    (:`then_0`
      ;;[1 1 1] This prevents firing by pressing fire multiple times, and force to wait until fire rate is reached.
      (set `self.primary fire rate` (- (`self.primary fire rate`) (`self.delta seconds`)))
      (if (<= (`self.primary fire rate`) 0.0)
        (`/Engine/EditorBlueprintResources/StandardMacros.Gate` true :!label _label
          (:`Exit`
            (set `self.primary fire rate` (`self.primary fire rate base`))
            ;;[1 1 1] If it doesn't have powerup, fire primary fire, otherwise fire power up fire.
            (if (not (`self.has power`))
              (`self.Primary Fire ` (`self.Projectile Spawn Location`))
              (else
                (`self.Power Up Fire` (`self.Power Shot Count`))))))))
    (:`then_1`
      (set `self.secondary fire rate` (- (`self.secondary fire rate`) (`self.delta seconds`)))
      (if (<= (`self.secondary fire rate`) 0.0)
        (`/Engine/EditorBlueprintResources/StandardMacros.Gate` true :!label _label_2
          (:`Exit`
            (set `self.secondary fire rate` (`self.secondary fire rate base`))
            (if (not (`self.has rockets`))
              (`self.Rocket Fire`))))))))

(event `InputAction|Secondary Fire`
  (params (Key :type "Key Structure"))
  ;[1 1 1] Projectile Control
  (:`Pressed`
    (goto _label_2 :!via `Open`))
  (:`Released`
    (goto _label_2 :!via `Close`)))

(fn `Get Direction`
  (params (Speed :type "Float (double-precision)") (Direction :type "Float (double-precision)"))
  (returns (`Return Direction` :type "Float (double-precision)"))
  (bind _delta_seconds (`self.delta seconds`))
  (bind _output_get (set `self.current speed` (* (`KismetMathLibrary.FInterpTo_Constant` Speed (* (* Direction (`self.movement speed`)) _delta_seconds) _delta_seconds 4.0) (`self.movement speed`))))
  (return _output_get))

(fn `Power Up Fire`
  (params (`Number of shots` :type Integer) (`Spawn Location` :type "SceneComponent Object Reference"))
  (locals (Offset :type Integer :default 0))
  (bind _returnvalue (`SceneComponent.K2_GetComponentToWorld` `Spawn Location`))
  (bind _returnvalue_2 (+ (`KismetMathLibrary.Conv_IntToDouble` (`local.Offset`)) 5.0))
  (set `local.Offset` (/ `Number of shots` 1))
  (for _ (range (+ `Number of shots` 1))
    (`|SpawnActorFromClass` "PlayerPawn_BP_C" (`KismetMathLibrary.MakeTransform` (`KismetMathLibrary.MakeVector` (.x (.location _returnvalue)) (.y (.location _returnvalue)) (+ (.z (.location _returnvalue)) _returnvalue_2)) (`KismetMathLibrary.MakeRotator` _returnvalue_2)) "AlwaysSpawn" "OverrideRootScale" null null)
    (set `local.Offset` (+ (`local.Offset`) 1))))

(fn `Primary Fire `
  (params (SpawnLocation :type "SceneComponent Object Reference"))
  (`|SpawnActorFromClass` "PlayerPawn_BP_C" (`KismetMathLibrary.MakeTransform` (`KismetMathLibrary.MakeVector` (.x (.location (`SceneComponent.K2_GetComponentToWorld` SpawnLocation))) (.y (.location (`SceneComponent.K2_GetComponentToWorld` SpawnLocation))) (+ (.z (.location (`SceneComponent.K2_GetComponentToWorld` SpawnLocation))) (`KismetMathLibrary.RandomFloatInRange` -70.0 70.0))) (.rotation (`SceneComponent.K2_GetComponentToWorld` SpawnLocation)) (.scale (`SceneComponent.K2_GetComponentToWorld` SpawnLocation))) "AlwaysSpawn" "OverrideRootScale" null null))

(fn `Rocket Fire`)

(fn `UserConstructionScript`)