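; Base projectile Blueprint that moves via a ProjectileMovement component and deals damage on overlap.
; The construction script applies the Speed variable as both initial and max speed, and sets the actor's scale from Scale.
; When the Cube component overlaps another Projectile_Base_BP, it applies Damage to that actor and destroys itself.
; That cast target is a placeholder marked for replacement with an enemy actor.
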(event `self.Cube.OnComponentBeginOverlap`
  (params (OverlappedComponent :type "PrimitiveComponent Object Reference") (OtherActor :type "Actor Object Reference") (OtherComp :type "PrimitiveComponent Object Reference") (OtherBodyIndex :type Integer) (bFromSweep :type Boolean) (SweepResult :type "HitResult Structure (by ref)"))
  ;[1 1 1] Collision events
  ;;[1 0.4137 0.0625] Replace me with enemy actor
  (bind _asprojectile_base_bp (cast `/Game/Blueprint/Projectile_Base_BP` OtherActor))
  (`GameplayStatics.ApplyDamage` _asprojectile_base_bp (`self.Damage`))
  (`self.K2_DestroyActor`))

(fn `UserConstructionScript`
  (bind _output_get (set `ProjectileMovementComponent.InitialSpeed` (`self.Speed`) (`self.ProjectileMovement`)))
  (set `ProjectileMovementComponent.MaxSpeed` _output_get (`self.ProjectileMovement`))
  (`self.SetActorScale3D` (`self.Scale`)))