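; Floating island actor that scrolls along negative Y as moving scenery, adorned with randomly chosen tree meshes.
; Its construction script adds a tree at each of three arrow transforms, then randomizes scale per axis and sets a fixed tilted rotation.
; Tick moves it a fixed step per frame, regardless of delta time.
; Once past OffscreenLeft, it waits briefly, asks GameMode_BP to spawn another island and destroys itself.
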(event `self.ReceiveTick`
  (params (DeltaSeconds :type "Float (single-precision)"))
  (bind (_returnvalue_x _returnvalue_y) (`KismetMathLibrary.BreakVector` (`SceneComponent.K2_GetComponentLocation` (`self.Scene`))))
  (if (< _returnvalue_y (`self.OffscreenLeft`))
    (`KismetSystemLibrary.Delay` (`KismetMathLibrary.RandomFloatInRange` 1.0 2.0))
    (bind _asgame_mode_bp (cast `/Game/Blueprint/GameMode_BP` (`GameplayStatics.GetGameMode`)))
    (`/Game/Blueprint/GameMode_BP.SpawnIsland` _asgame_mode_bp)
    (`self.K2_DestroyActor`)
    (else
      (`SceneComponent.K2_AddWorldOffset` (`self.Scene`) (0.0 -20.0 0.0) false false))))

(fn `Set Spawn Points`
  (set `self.Spawn Points` (`|MakeArray` (`SceneComponent.GetRelativeTransform` (`self.Arrow`)) (`SceneComponent.GetRelativeTransform` (`self.Arrow1`)) (`SceneComponent.GetRelativeTransform` (`self.Arrow2`)))))

(fn `Spawn Trees`
  (for _index (range (`KismetArrayLibrary.Array_Length` (`self.Spawn Points`)))
    (bind _returnvalue (`AddComponent|NODE_AddStaticMeshComponent-0` :`RelativeTransform` (`|GetArrayItem` (`self.Spawn Points`) _index)))
    (`StaticMeshComponent.SetStaticMesh` _returnvalue (`|GetArrayItem` (`self.Trees`) (`KismetMathLibrary.RandomIntegerInRange` 0 (- (`KismetArrayLibrary.Array_Length` (`self.Trees`)) 1))))))

(fn `UserConstructionScript`
  (bind _returnvalue (`KismetMathLibrary.RandomFloatInRange` 0.3 1.0))
  (`self.Set Spawn Points`)
  (`self.Spawn Trees`)
  (`self.SetActorScale3D` (`KismetMathLibrary.MakeVector` _returnvalue _returnvalue _returnvalue))
  (`self.K2_SetActorRotation` (struct :`Pitch` 15.0 :`Yaw` -50.0 :`Roll` -15.0)))