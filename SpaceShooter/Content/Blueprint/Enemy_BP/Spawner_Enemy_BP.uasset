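; Enemy wave spawner that runs a fixed six-wave sequence, then calls the game mode's end screen.
; A looping timer starts the next wave once the game mode reports no live enemies and the spawner is ready.
; Each wave passes its enemy count to the game mode and draws random classes from one of three reused pools.
; Enemies spawn at the spawner's X, with random Y and Z within game mode bounds.
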(event `self.ReceiveBeginPlay`
  ;[1 1 1] Event beginplay - spawn wave
  (bind _asgame_mode_bp (cast `/Game/Blueprint/GameMode_BP` (`GameplayStatics.GetGameMode`)))
  (set `self.GameMode_BP` _asgame_mode_bp)
  (bind _returnvalue (`KismetSystemLibrary.K2_SetTimer` null "Wave Check" 0.5 true))
  (set `self.Wave Timer` _returnvalue))

(event `Wave Check`
  (bind _output (`|GetArrayItem` (`self.Wave Enemy Count`) (`self.Wave Index`)))
  (bind _output_2 (`|GetArrayItem` (`self.Wave Enemy Count`) (`self.Wave Index`)))
  (bind _output_3 (`|GetArrayItem` (`self.Wave Enemy Count`) (`self.Wave Index`)))
  (bind _output_4 (`|GetArrayItem` (`self.Wave Enemy Count`) (`self.Wave Index`)))
  (bind _output_5 (`|GetArrayItem` (`self.Wave Enemy Count`) (`self.Wave Index`)))
  (bind _output_6 (`|GetArrayItem` (`self.Wave Enemy Count`) (`self.Wave Index`)))
  (if (and (== (`/Game/Blueprint/GameMode_BP.live enemies` (`self.GameMode_BP`)) 0) (`self.IsWaveReady`))
    (switch `int` (`self.Wave Index`)
      (:`Default`
        (`/Game/Blueprint/GameMode_BP.GameEndScreen` (`self.GameMode_BP`) "/Game/Blueprint/UI/QuitMenu.QuitMenu_C"))
      (:`0`
        (`self.Begin Wave` _output_5)
        (`self.Spawn Wave` _output_5 (`self.Wave Enemies 1`))
        (set `self.Wave Index` (+ (`self.Wave Index`) 1) :!label _label))
      (:`1`
        (`self.Begin Wave` _output_3)
        (`self.Spawn Wave` _output_3 (`self.Wave Enemies 2`))
        (goto _label))
      (:`2`
        (`self.Begin Wave` _output_2)
        (`self.Spawn Wave` _output_2 (`self.Wave Enemies 3`))
        (goto _label))
      (:`3`
        (`self.Begin Wave` _output_4)
        (`self.Spawn Wave` _output_4 (`self.Wave Enemies 2`))
        (goto _label))
      (:`4`
        (`self.Begin Wave` _output_6)
        (`self.Spawn Wave` _output_6 (`self.Wave Enemies 1`))
        (goto _label))
      (:`5`
        (`self.Begin Wave` _output)
        (`self.Spawn Wave` _output (`self.Wave Enemies 3`))
        (goto _label)))))

(fn `Begin Wave`
  (params (`Wave total` :type Integer))
  (set `self.IsWaveReady` false)
  (set `self.Wave Active` 0)
  (set `/Game/Blueprint/GameMode_BP.max waves` `Wave total` (`self.GameMode_BP`))
  (set `/Game/Blueprint/GameMode_BP.active wave` `Wave total` (`self.GameMode_BP`)))

(fn `Spawn Wave`
  (params (`Wave Total` :type Integer) (`Wave Enemies` :type "Array of /Game/Blueprint/Enemy_BP/Enemy_Base_BP Class Reference"))
  (locals (WaveTotal :type Integer))
  (bind _gamemode_bp (`self.GameMode_BP`))
  (bind (_enemy_spawn_location_min_x _enemy_spawn_location_min_y _enemy_spawn_location_min_z) (`KismetMathLibrary.BreakVector` (`/Game/Blueprint/GameMode_BP.enemy spawn location min` _gamemode_bp)))
  (bind (_enemy_spawn_location_max_x _enemy_spawn_location_max_y _enemy_spawn_location_max_z) (`KismetMathLibrary.BreakVector` (`/Game/Blueprint/GameMode_BP.enemy spawn location max` _gamemode_bp)))
  (set `local.WaveTotal` `Wave Total`)
  (for _ (range (+ (+ (`local.WaveTotal`) (`self.Wave Active`)) 1))
    (if (> (`local.WaveTotal`) (`self.Wave Active`))
      (if true
        (`|SpawnActorFromClass` (`|GetArrayItem` `Wave Enemies` (`KismetMathLibrary.RandomInteger` (`KismetArrayLibrary.Array_Length` `Wave Enemies`))) (`KismetMathLibrary.MakeTransform` (`KismetMathLibrary.MakeVector` (.x (.location (`self.GetTransform`))) (`KismetMathLibrary.RandomFloatInRange` _enemy_spawn_location_min_y _enemy_spawn_location_max_y) (`KismetMathLibrary.RandomFloatInRange` _enemy_spawn_location_min_z _enemy_spawn_location_max_z))) "Undefined" "OverrideRootScale" null null)
        (set `self.Wave Active` (+ (`self.Wave Active`) 1)))
      (else
        (set `self.IsWaveReady` true)))))

(fn `UserConstructionScript`)