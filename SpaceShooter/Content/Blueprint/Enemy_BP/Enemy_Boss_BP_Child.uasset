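; Child Blueprint variant of an enemy boss that repeatedly fires projectiles from two muzzle points.
; Tick runs the parent logic, then uses a Delay of FireRate as a repeating fire timer.
; Each shot spawns ProjectileEnemy_BP at the Top and Bottom transforms with fixed damage and negative-Y velocity, playing one EnemyShot sound at the world origin.
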(event `self.ReceiveTick`
  (params (DeltaSeconds :type "Float (single-precision)"))
  (`parent.ReceiveTick` DeltaSeconds)
  (`KismetSystemLibrary.Delay` (`self.Fire Rate`))
  (`|ExecutionSequence`
    (:`then_0`
      (`|SpawnActorFromClass` "/Game/Blueprint/Enemy_BP/ProjectileENemy_BP.ProjectileEnemy_BP_C" (`SceneComponent.K2_GetComponentToWorld` (`self.Top`)) "Undefined" "OverrideRootScale" null 1.0 (0.0 -2000.0 0.0) (1.0 1.0 1.0) null)
      (`GameplayStatics.PlaySoundAtLocation` "/Game/Audio/EnemyShot.EnemyShot"))
    (:`then_1`
      (`|SpawnActorFromClass` "/Game/Blueprint/Enemy_BP/ProjectileENemy_BP.ProjectileEnemy_BP_C" (`SceneComponent.K2_GetComponentToWorld` (`self.Bottom`)) "Undefined" "OverrideRootScale" null 1.0 (0.0 -2000.0 0.0) (1.0 1.0 1.0) null))))

(fn `UserConstructionScript`
  (`parent.UserConstructionScript`))