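; Child enemy Blueprint, derived from its parent enemy, that repeatedly fires projectiles.
; Tick runs the parent logic, then uses a Delay of FireRate as a repeating fire timer.
; Each shot spawns ProjectileEnemy_BP at the ProjectileSpawn transform with fixed damage, negative-Y speed and enlarged scale, then plays EnemyShot at the world origin.
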(event `self.ReceiveTick`
  (params (DeltaSeconds :type "Float (single-precision)"))
  (`parent.ReceiveTick` DeltaSeconds)
  (`KismetSystemLibrary.Delay` (`self.Fire Rate`))
  (`|SpawnActorFromClass` "/Game/Blueprint/Enemy_BP/ProjectileENemy_BP.ProjectileEnemy_BP_C" (`SceneComponent.K2_GetComponentToWorld` (`self.ProjectileSpawn`)) "Undefined" "OverrideRootScale" null 10.0 (0.0 -2000.0 0.0) (2.0 2.0 2.0) null)
  (`GameplayStatics.PlaySoundAtLocation` "/Game/Audio/EnemyShot.EnemyShot"))

(fn `UserConstructionScript`
  (`parent.UserConstructionScript`))