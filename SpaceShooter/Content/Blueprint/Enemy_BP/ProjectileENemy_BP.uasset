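; Enemy projectile actor that flies along its local axes at a set speed and damages the player pawn on impact.
; Tick moves it with a swept local offset, and the construction script applies a configurable scale.
; On a mesh hit against PlayerPawn_BP it applies damage, spawns a hit particle, asks GameMode_BP for a camera shake and destroys itself.
; Any other hit simply destroys it.
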(event `self.ReceiveTick`
  (params (DeltaSeconds :type "Float (single-precision)"))
  ;[1 1 1] Move Projectile
  (`self.K2_AddActorLocalOffset` (* (`self.Speed`) DeltaSeconds) true))

(event `self.ProjectileMesh.OnComponentHit`
  (params (HitComponent :type "PrimitiveComponent Object Reference") (OtherActor :type "Actor Object Reference") (OtherComp :type "PrimitiveComponent Object Reference") (NormalImpulse :type "Vector Structure") (Hit :type "HitResult Structure (by ref)"))
  ;[1 1 1] Collision events
  (bind _asplayer_pawn_bp (cast `/Game/Blueprint/Player_BP/PlayerPawn_BP` OtherActor)
    (:`then`
      (`GameplayStatics.ApplyDamage` _asplayer_pawn_bp (`self.Damage`))
      ;;[1 1 1] Explosion particle
      (`GameplayStatics.SpawnEmitterAtLocation` "/Game/Art/Particles/Particle_Hit_Enemy.Particle_Hit_Enemy" (`self.K2_GetActorLocation`))
      ;;[1 1 1] Camera Shake
      (bind _asgame_mode_bp (cast `/Game/Blueprint/GameMode_BP` (`GameplayStatics.GetGameMode`)))
      (`/Game/Blueprint/GameMode_BP.CameraShake` _asgame_mode_bp "/Game/Blueprint/Camera_Shake_BP.Camera_Shake_BP_C")
      (`self.K2_DestroyActor`))
    (:`CastFailed`
      (`self.K2_DestroyActor`))))

(fn `UserConstructionScript`
  (`self.SetActorScale3D` (`self.Scale`)))