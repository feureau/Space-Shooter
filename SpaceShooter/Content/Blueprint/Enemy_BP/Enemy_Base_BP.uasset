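; Base enemy Blueprint that registers in the game mode's live enemy count, sweeps in on a spawn timeline, then moves back and forth at random speed.
; Hitting anything except another enemy reverses its direction; hitting the player also deals damage and kills the enemy.
; Damage that empties health shares that death path: decrement the count, add score, maybe drop a random pickup, play effects and destroy.
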(event `self.ReceiveBeginPlay`
  (bind _spawnlocation (`self.SpawnLocation`))
  ;[1 1 1] Add this enemy to live enemies count in game mode
  (bind _asgame_mode_bp (cast `/Game/Blueprint/GameMode_BP` (`GameplayStatics.GetGameMode`)))
  (bind _output_get (set `self.GameMode_BP` _asgame_mode_bp))
  (set `/Game/Blueprint/GameMode_BP.live enemies` (+ (`/Game/Blueprint/GameMode_BP.live enemies` _output_get) 1) (`self.GameMode_BP`))
  (set `self.MoveDirection` (`KismetMathLibrary.RandomBool`))
  (set `self.MoveSpeed` (`KismetMathLibrary.RandomFloatInRange` 500.0 1000.0))
  (set `self.SweepIn` (`KismetMathLibrary.RandomFloatInRange` 1200.0 1700.0))
  ;[1 1 1] Spawn Animation
  (set `self.SpawnLocation` (`self.K2_GetActorLocation`))
  (bind (_direction _speed) (`Timeline|SpawnAnimation_Timeline`)
    (:`Update`
      (`self.K2_SetActorLocation` (`KismetMathLibrary.VLerp` _spawnlocation (- _spawnlocation (`KismetMathLibrary.MakeVector` 0.0 (`self.SweepIn`))) _speed)))
    (:`Finished`
      (set `self.MoveEnabled` true))))

(event `self.ReceiveTick`
  (params (DeltaSeconds :type "Float (single-precision)"))
  ;[1 1 1] Movement
  (if (`self.MoveEnabled`)
    (`self.K2_SetActorLocation` (+ (`self.K2_GetActorLocation`) (* (`KismetMathLibrary.GreaterGreater_VectorRotator` (`KismetMathLibrary.MakeVector` 0.0 0.0 (* (`self.MoveSpeed`) (`KismetMathLibrary.SelectFloat` 1.0 -1.0 (`self.MoveDirection`))))) DeltaSeconds)) true)))

(event `self.ReceiveHit`
  (params (MyComp :type "PrimitiveComponent Object Reference") (Other :type "Actor Object Reference") (OtherComp :type "PrimitiveComponent Object Reference") (bSelfMoved :type Boolean) (HitLocation :type "Vector Structure") (HitNormal :type "Vector Structure") (NormalImpulse :type "Vector Structure") (Hit :type "HitResult Structure (by ref)"))
  (bind _pickups (`self.Pickups`))
  ;[1 1 1] Death
  (cast `/Game/Blueprint/Enemy_BP/Enemy_Base_BP` Other
    (:`CastFailed`
      (set `self.MoveDirection` (not (`self.MoveDirection`)))
      (bind _asplayer_pawn_bp (cast `/Game/Blueprint/Player_BP/PlayerPawn_BP` Other))
      (`GameplayStatics.ApplyDamage` _asplayer_pawn_bp 50.0)
      (set `/Game/Blueprint/GameMode_BP.live enemies` (- (`/Game/Blueprint/GameMode_BP.live enemies` (`self.GameMode_BP`)) 1) (`self.GameMode_BP`) :!label _label)
      (`/Game/Blueprint/GameMode_BP.AddScore` (`self.GameMode_BP`) 10)
      (if (<= (`KismetMathLibrary.RandomFloatInRange` 0.0 1.0) (`self.DropRate`))
        (`|SpawnActorFromClass` (`|GetArrayItem` _pickups (`KismetMathLibrary.RandomIntegerInRange` 0 (`KismetArrayLibrary.Array_LastIndex` _pickups))) (`self.GetTransform`) "Undefined" "OverrideRootScale" null null))
      (`GameplayStatics.SpawnEmitterAtLocation` "/Game/Art/Particles/Particle_Death_Enemy.Particle_Death_Enemy" (`self.K2_GetActorLocation`))
      (`GameplayStatics.PlaySound2D` "/Game/Audio/Explosion.Explosion")
      (`self.K2_DestroyActor`))))

(event `self.ReceiveAnyDamage`
  (params (Damage :type "Float (single-precision)") (DamageType :type "DamageType Object Reference") (InstigatedBy :type "Controller Object Reference") (DamageCauser :type "Actor Object Reference"))
  ;[1 1 1] Death
  (bind _output_get (set `self.Health` (`KismetMathLibrary.FClamp` (- (`self.Health`) Damage) 0.0 (`self.MaxHealth`))))
  (if (<= _output_get 0.0)
    (goto _label)))

(fn `UserConstructionScript`
  (set `self.Health` (`self.MaxHealth`)))