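; Base Blueprint for player projectiles that damage enemies on contact.
; The construction script sets the actor scale and applies the Speed variable to the projectile movement's initial and max speed.
; When the cube overlaps an enemy, it applies damage, spawns a hit particle and requests a camera shake through the game mode.
; The projectile destroys itself after a hit or on overlapping any non-enemy actor.
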(event `self.Cube.OnComponentBeginOverlap`
  (params (OverlappedComponent :type "PrimitiveComponent Object Reference") (OtherActor :type "Actor Object Reference") (OtherComp :type "PrimitiveComponent Object Reference") (OtherBodyIndex :type Integer) (bFromSweep :type Boolean) (SweepResult :type "HitResult Structure (by ref)"))
  ;[1 1 1] Collision events
  (bind _asenemy_base_bp (cast `/Game/Blueprint/Enemy_BP/Enemy_Base_BP` OtherActor)
    (:`then`
      (`GameplayStatics.ApplyDamage` _asenemy_base_bp (`self.Damage`))
      (`GameplayStatics.SpawnEmitterAtLocation` "/Game/Art/Particles/Particle_Hit_Player.Particle_Hit_Player" (`self.K2_GetActorLocation`))
      ;;[1 1 1] Camera Shake
      (bind _asgame_mode_bp (cast `/Game/Blueprint/GameMode_BP` (`GameplayStatics.GetGameMode`)))
      (`/Game/Blueprint/GameMode_BP.CameraShake` _asgame_mode_bp "/Game/Blueprint/Camera_Shake_BP.Camera_Shake_BP_C")
      (`self.K2_DestroyActor`))
    (:`CastFailed`
      (`self.K2_DestroyActor`))))

(fn `UserConstructionScript`
  (bind _output_get (set `ProjectileMovementComponent.InitialSpeed` (`self.Speed`) (`self.ProjectileMovement`)))
  (set `ProjectileMovementComponent.MaxSpeed` _output_get (`self.ProjectileMovement`))
  (`self.SetActorScale3D` (`self.Scale`)))