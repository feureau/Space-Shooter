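; Player ship pawn for a shooter: adds the HUD outside the menu map, flies in on a spawn timeline and moves on the Y/Z plane.
; Tick drives interpolated movement, banking and fire-rate countdowns.
; Input opens gates that those countdowns pulse, firing randomised primary shots or multi-shot power-ups, plus rockets when owned.
; Projectile hits knock the ship back; lethal damage notifies GameMode, destroys the pawn and restores the scene camera.
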(event `self.ReceiveBeginPlay`
  (bind _spawn_location (`self.spawn location`))
  (set `self.health` (`self.max health`))
  ;[1 1 1] only display in-game HUD if level is not "Menu"
  (bind _returnvalue (`GameplayStatics.GetCurrentLevelName` true))
  (if (`KismetStringLibrary.NotEqual_StrStr` _returnvalue "Menu_Map")
    ;[1 1 1] Display in-game HUD
    (bind _returnvalue_2 (`|CreateWidget` "/Game/Blueprint/UI/HUD.HUD_C"))
    (bind _output_get (set `self.HUD Reference` _returnvalue_2))
    (`UserWidget.AddToViewport` _output_get 0))
  (set `self.pitch` (.pitch (`SceneComponent.RelativeRotation` (`self.Player Mesh`))))
  (set `self.spawn location` (`self.K2_GetActorLocation`))
  ;[1 1 1] Spawn Animation
  (bind (_direction _spawn) (`Timeline|Spawn Animation`)
    (:`Update`
      (`self.K2_SetActorLocation` (`KismetMathLibrary.VLerp` _spawn_location (+ _spawn_location (0.0 1000.0 0.0)) _spawn))
      (`SceneComponent.K2_SetRelativeRotation` (`self.Player Mesh`) (`KismetMathLibrary.RLerp` (struct) (`KismetMathLibrary.MakeRotator` 0.0 (+ (`self.Animation pitch`) (`self.pitch`))) _spawn) false false)
      ;[1 1 1] Get the active camera
      (bind _outactors (`GameplayStatics.GetAllActorsOfClass` "/Script/Engine.CameraActor"))
      (for _array_element _outactors
        (if (`ActorComponent.IsActive` (`CameraActor.CameraComponent` _array_element))
          (set `self.Scene Camera` _array_element))))))

(event `self.ReceiveTick`
  (params (DeltaSeconds :type "Float (single-precision)"))
  (set `self.delta seconds` DeltaSeconds)
  (if (`self.movement enabled`)
    (`self.Fire Rate Control`)
    (`|ExecutionSequence`
      (:`then_0`
        (bind _return_direction (`self.Get Direction` (`self.vertical speed`) (`self.GetInputAxisValue`)))
        (set `self.vertical speed` _return_direction))
      (:`then_1`
        (bind _return_direction_2 (`self.Get Direction` (`self.horizontal speed`) (`self.GetInputAxisValue`)))
        (set `self.horizontal speed` _return_direction_2))
      (:`then_2`
        (`self.K2_SetActorLocation` (+ (`self.K2_GetActorLocation`) (`KismetMathLibrary.MakeVector` 0.0 0.0 (`self.vertical speed`))) true)
        (`self.K2_SetActorLocation` (+ (`self.K2_GetActorLocation`) (`KismetMathLibrary.MakeVector` 0.0 (`self.horizontal speed`))) true)
        (set `self.vertical speed` (`self.GetInputAxisValue`))
        (set `self.horizontal speed` (`self.GetInputAxisValue`))
        ;[1 1 1] so the actor only rotates if the player is alive
        (if (> (`self.health`) 0.0)
          (`self.K2_SetActorRotation` (`KismetMathLibrary.RInterpTo` (`self.K2_GetActorRotation`) (`KismetMathLibrary.MakeRotator` (* (`self.vertical speed`) -45.0) 0.0 90.0) (`self.delta seconds`) 5.0)))))))

(event `InputAction|Primary Fire`
  (params (Key :type "Key Structure"))
  ;[1 1 1] Projectile Control
  (:`Pressed`
    (goto _label :!via `Open`))
  (:`Released`
    (goto _label :!via `Close`)))

(event `Fire Rate Control`
  ;[1 1 1] Projectile Control
  (`|ExecutionSequence`
    (:`then_0`
      ;;[1 1 1] This prevents firing by pressing fire multiple times, and force to wait until fire rate is reached.
      (set `self.primary fire rate` (- (`self.primary fire rate`) (`self.delta seconds`)))
      (if (<= (`self.primary fire rate`) 0.0)
        (`/Engine/EditorBlueprintResources/StandardMacros.Gate` true :!label _label
          (:`Exit`
            (set `self.primary fire rate` (`self.primary fire rate base`))
            ;;[1 1 1] If it doesn't have powerup, fire primary fire, otherwise fire power up fire.
            (if (not (`self.has power`))
              (`self.Primary Fire ` (`self.Projectile Spawn Location`))
              (else
                (`self.Power Up Fire` (`self.Power Shot Count`) (`self.Projectile Spawn Location`))))
            (`GameplayStatics.PlaySoundAtLocation` "/Game/Audio/EnemyShot.EnemyShot")))))
    (:`then_1`
      (set `self.secondary fire rate` (- (`self.secondary fire rate`) (`self.delta seconds`)))
      (if (<= (`self.secondary fire rate`) 0.0)
        (`/Engine/EditorBlueprintResources/StandardMacros.Gate` true :!label _label_2
          (:`Exit`
            (set `self.secondary fire rate` (`self.secondary fire rate base`))
            (if (`self.has rockets`)
              (`self.Rocket Fire` (`self.Rocket shot count`) (`self.Projectile Spawn Location`)))))))))

(event `InputAction|Secondary Fire`
  (params (Key :type "Key Structure"))
  ;[1 1 1] Projectile Control
  (:`Pressed`
    (goto _label_2 :!via `Open`))
  (:`Released`
    (goto _label_2 :!via `Close`)))

(event `self.ReceiveAnyDamage`
  (params (Damage :type "Float (single-precision)") (DamageType :type "DamageType Object Reference") (InstigatedBy :type "Controller Object Reference") (DamageCauser :type "Actor Object Reference"))
  (bind _output_get (set `self.health` (`KismetMathLibrary.FClamp` (- (`self.health`) Damage) 0.0 (`self.max health`))))
  (if (<= _output_get 0.0)
    (bind _asgame_mode_bp (cast `/Game/Blueprint/GameMode_BP` (`GameplayStatics.GetGameMode`)))
    (bind _output_get_2 (set `self.Game Mode BP` _asgame_mode_bp))
    (set `/Game/Blueprint/GameMode_BP.is player dead` true _output_get_2)
    (`/Game/Blueprint/GameMode_BP.AllEnemiesDefeated` (`self.Game Mode BP`) "/Game/Blueprint/UI/QuitMenu.QuitMenu_C")
    (`GameplayStatics.SpawnEmitterAtLocation` "/Game/Art/Particles/Particle_Death_Player.Particle_Death_Player" (`self.K2_GetActorLocation`))
    (`self.K2_DestroyActor`)
    (`PlayerController.SetViewTargetWithBlend` (`GameplayStatics.GetPlayerController` 0) (`self.Scene Camera`) 0.0 "VTBlend_Linear" 0.0 false)))

(event `self.Ship collider.OnComponentHit`
  (params (HitComponent :type "PrimitiveComponent Object Reference") (OtherActor :type "Actor Object Reference") (OtherComp :type "PrimitiveComponent Object Reference") (NormalImpulse :type "Vector Structure") (Hit :type "HitResult Structure (by ref)"))
  (cast `/Game/Blueprint/Enemy_BP/ProjectileENemy_BP` OtherActor
    (:`then`
      (set `self.horizontal speed` (* (* (`KismetMathLibrary.Abs` (`self.horizontal speed`)) 15.0) (.y Hit_Normal)))
      (set `self.vertical speed` (* (.z Hit_Normal) (* 15.0 (`KismetMathLibrary.Abs` (`self.vertical speed`))))))
    (:`CastFailed`
      (cast `/Game/Blueprint/Enemy_BP/Enemy_Base_BP` OtherActor))))

(fn `Get Direction`
  (params (Speed :type "Float (double-precision)") (Direction :type "Float (double-precision)"))
  (returns (`Return Direction` :type "Float (double-precision)"))
  (bind _output_get (set `self.current speed` (* (`KismetMathLibrary.FInterpTo_Constant` Speed (* Direction (`self.movement speed`)) (`self.delta seconds`) 4.0) (`self.movement speed`))))
  (return _output_get))

(fn `Power Up Fire`
  (params (`Number of shots` :type Integer) (`Spawn Location` :type "SceneComponent Object Reference"))
  (locals (Offset :type Integer :default 0) (`Projectile spread total degrees` :type "Float (double-precision)" :default 25.0))
  (bind _returnvalue (`SceneComponent.K2_GetComponentToWorld` `Spawn Location`))
  (bind _projectile_spread_total_degrees (`local.Projectile spread total degrees`))
  (bind _returnvalue_2 (/ _projectile_spread_total_degrees -2.0))
  (for _index (range (+ `Number of shots` 1))
    (`|SpawnActorFromClass` "/Game/Blueprint/Player_BP/PoweredProjectile_BP_Child.PoweredProjectile_BP_Child_C" (`KismetMathLibrary.MakeTransform` (`KismetMathLibrary.MakeVector` (.x (.location _returnvalue)) (.y (.location _returnvalue)) (.z (.location _returnvalue))) (`KismetMathLibrary.MakeRotator` (+ (* _index (+ _returnvalue_2 (/ _projectile_spread_total_degrees (`KismetMathLibrary.Conv_IntToDouble` `Number of shots`)))) _returnvalue_2 _projectile_spread_total_degrees))) "AlwaysSpawn" "OverrideRootScale" null null)
    (set `local.Offset` (+ 0 0))))

(fn `Primary Fire `
  (params (SpawnLocation :type "SceneComponent Object Reference"))
  (`|SpawnActorFromClass` "/Game/Blueprint/Player_BP/Primary_Projectile_BP_Child.Primary_Projectile_BP_Child_C" (`KismetMathLibrary.MakeTransform` (`KismetMathLibrary.MakeVector` (.x (.location (`SceneComponent.K2_GetComponentToWorld` SpawnLocation))) (.y (.location (`SceneComponent.K2_GetComponentToWorld` SpawnLocation))) (+ (.z (.location (`SceneComponent.K2_GetComponentToWorld` SpawnLocation))) (`KismetMathLibrary.RandomFloatInRange` -140.0 140.0))) (`KismetMathLibrary.MakeRotator` (+ (.roll (.rotation (`SceneComponent.K2_GetComponentToWorld` SpawnLocation))) (`KismetMathLibrary.RandomFloatInRange` -10.0 10.0)) (.pitch (.rotation (`SceneComponent.K2_GetComponentToWorld` SpawnLocation))) (.yaw (.rotation (`SceneComponent.K2_GetComponentToWorld` SpawnLocation)))) (.scale (`SceneComponent.K2_GetComponentToWorld` SpawnLocation))) "AlwaysSpawn" "OverrideRootScale" null null))

(fn `Rocket Fire`
  (params (`Number of Shots` :type Integer) (`Spawn Location` :type "SceneComponent Object Reference"))
  (locals (Offset :type Integer :default 0))
  (bind _returnvalue (* (`local.Offset`) 5.0))
  (set `local.Offset` (/ (+ `Number of Shots` 1) -1))
  (for _ (range (+ `Number of Shots` 1))
    (`|SpawnActorFromClass` "/Game/Blueprint/Player_BP/RocketProjectile_BP_Child.RocketProjectile_BP_Child_C" (`KismetMathLibrary.MakeTransform` (`KismetMathLibrary.MakeVector` (.x (.location (`SceneComponent.K2_GetComponentToWorld` `Spawn Location`))) (.y (.location (`SceneComponent.K2_GetComponentToWorld` `Spawn Location`))) (+ (.z (.location (`SceneComponent.K2_GetComponentToWorld` `Spawn Location`))) _returnvalue)) (`KismetMathLibrary.MakeRotator` _returnvalue)) "AlwaysSpawn" "OverrideRootScale" null null)
    (set `local.Offset` (+ (`local.Offset`) 4))))

(fn `UserConstructionScript`)